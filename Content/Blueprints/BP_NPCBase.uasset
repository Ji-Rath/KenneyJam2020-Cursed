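; Base NPC Blueprint with an Emotion widget component that displays a texture for a given duration.
; Every tick, the widget smoothly turns toward the BP_Player camera, interpolating toward the look-at rotation from the NPC's location and applying only yaw so it stays upright.
; ShowEmotion passes the texture and duration through to the component's WBP_Emotion widget.
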(event EventTick
  (params (DeltaSeconds :type Float%20%28single-precision%29))
  (CallFunction|UpdateEmotionWidget))

(fn ConstructionScript)

(fn UpdateEmotionWidget
  (bind _emotion (Variables|Default|GetEmotion))
  (bind _asbp_player (Utilities|Casting|CastToBP_Player (Game|GetPlayerCharacter 0)))
  (Transformation|SetWorldRotation _emotion (Math|Rotator|MakeRotator 0.0 0.0 (.yaw (Math|Interpolation|RInterpTo (Transformation|GetWorldRotation _emotion) (Math|Rotator|FindLookatRotation (Transformation|GetActorLocation) (Transformation|GetWorldLocation (Variables|/Game/Blueprints/BP_Player.BP_Player_C|GetCamera _asbp_player))) (Utilities|Time|GetWorldDeltaSeconds) 5.0))) false false))

(fn ShowEmotion
  (params (Texture :type Texture%202D%20Object%20Reference) (Duration :type Float%20%28single-precision%29))
  (bind _aswbp_emotion (Utilities|Casting|CastToWBP_Emotion (UserInterface|GetUserWidgetObject (Variables|Default|GetEmotion))))
  (Default|ShowEmotion _aswbp_emotion Texture Duration))