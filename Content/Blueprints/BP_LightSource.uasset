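; BP_LightSource is a light actor that drives the day cycle by rotating its light and refreshing the sky material.
; A looping timer starts each transition and advances the cyclic TimeOfDay phase in BP_CursedGameMode, printing the new value.
; While the transition flag is set, Tick pitches the light in fixed per-frame steps, independent of delta time, until roughly a quarter turn completes.
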(event EventTick
  (params (DeltaSeconds :type Float%20%28single-precision%29))
  (if (Variables|Default|GetbUpdateDay)
    (Transformation|AddLocalRotation (Variables|Default|GetLightComponent) "-0.100000,0.000000,0.000000" false false)
    (Variables|Default|SetRotationCount (+ (Variables|Default|GetRotationCount) 0.1))
    (Default|RefreshMaterial (Variables|Default|GetSkyRef))
    (if (>= (+ (Variables|Default|GetRotationCount) 0.1) 9e+01)
      (Variables|Default|SetbUpdateDay false)
      (Variables|Default|SetRotationCount 0.0))))

(event EventBeginPlay
  (Utilities|Time|SetTimerbyFunctionName 0 "UpdateDay" 1e+01 true))

(fn ConstructionScript)

(fn UpdateDay
  (Variables|Default|SetbUpdateDay true)
  (bind _asbp_cursed_game_mode (Utilities|Casting|CastToBP_CursedGameMode (Game|GetGameMode)))
  (bind _result (Math|Integer|IncrementInt (Variables|/Script/KenneyJam2020.KenneyJam2020GameModeBase|GetTimeOfDay _asbp_cursed_game_mode))
    (:%20%20
      (if (> _result 3)
        (Variables|/Script/KenneyJam2020.KenneyJam2020GameModeBase|SetTimeOfDay _asbp_cursed_game_mode 0))
      (Development|PrintString (Utilities|String|ToString(Integer) (Variables|/Script/KenneyJam2020.KenneyJam2020GameModeBase|GetTimeOfDay _asbp_cursed_game_mode))))))