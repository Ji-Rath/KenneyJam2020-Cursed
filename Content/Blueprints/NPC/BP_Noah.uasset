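; Noah NPC Blueprint whose only active logic responds to the VillagerDeath event.
; It creates a level sequence player for SallyDeadSequence using the cursed game mode's settings and stores it as that game mode's CurrentSequence.
; After a player-character cast succeeds, it binds an event to the sequence's finish, though no Play call or handler body appears here.
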(event EventBeginPlay)

(event Collision|EventActorBeginOverlap
  (params (OtherActor :type Actor%20Object%20Reference)))

(event EventTick
  (params (DeltaSeconds :type Float%20%28single-precision%29))
  (|CallParentFunction DeltaSeconds) ; This node is disabled and will not be called.\nDrag off pins to build functionality.
)

(event EventVillagerDeath
  (bind _asbp_cursed_game_mode (Utilities|Casting|CastToBP_CursedGameMode (Game|GetGameMode)))
  (bind _returnvalue (Sequencer|Player|CreateLevelSequencePlayer "/Game/Sequences/SallyDeadSequence.SallyDeadSequence" (Variables|/Game/Blueprints/BP_CursedGameMode.BP_CursedGameMode_C|GetMainSequences _asbp_cursed_game_mode)))
  (bind _output_get (Variables|/Game/Blueprints/BP_CursedGameMode.BP_CursedGameMode_C|SetCurrentSequence _asbp_cursed_game_mode _returnvalue))
  (bind _asbp_player (Utilities|Casting|CastToBP_Player (Game|GetPlayerCharacter 0)))
  (EventDispatchers|BindEventtoOnFinished _output_get (EventDispatchers|CreateEvent _asbp_player :!event Death)))

(fn ConstructionScript
  (|CallParentFunction))