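; AI controller for NPCs that starts the BT_NPC behavior tree when it possesses a pawn.
; It then casts the pawn to BP_NPCBase and copies that NPC's house location, work location and friend reference into the blackboard as object values.
; The tree thus gets per-NPC defaults from variables on each character.
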(event EventPossess
  (params (PossessedPawn :type Pawn%20Object%20Reference))
  (bind _returnvalue (AI|GetBlackboard 0))
  (AI|RunBehaviorTree "/Game/Blueprints/AI/BT_NPC.BT_NPC")
  (bind _asbp_npcbase (Utilities|Casting|CastToBP_NPCBase (Pawn|GetControlledPawn)))
  ;[1 1 1] Set appropriate BB values to default values on NPC
  (AI|Components|Blackboard|SetValueasObject _returnvalue (Utilities|Name|MakeLiteralName "HouseLocation") (Variables|/Script/KenneyJam2020.NPCBase|GetHouseLocation _asbp_npcbase))
  (AI|Components|Blackboard|SetValueasObject _returnvalue (Utilities|Name|MakeLiteralName "WorkLocation") (Variables|/Script/KenneyJam2020.NPCBase|GetWorkLocation _asbp_npcbase))
  (AI|Components|Blackboard|SetValueasObject _returnvalue (Utilities|Name|MakeLiteralName "FriendRef") (Variables|/Script/KenneyJam2020.NPCBase|GetFriendRef _asbp_npcbase)))

(fn ConstructionScript)